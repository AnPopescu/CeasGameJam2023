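; Spawner actor that drops randomly scaled BP_SandChunk actors along a horizontal span between two limit markers.
; The construction script adds the left and right marker meshes at mirrored Y offsets from DistanceFromCenter, and ChangeDistanceFromCenter repositions them.
; After a short BeginPlay delay, it enables player input and starts a looping SpawnRate timer.
; Each tick of that timer spawns a chunk at a random world Y between the markers.
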(event Custom|SpawnSand
  (bind _returnvalue (Transformation|GetActorLocation))
  (bind _returnvalue_2 (Math|Random|RandomFloatinRange 0.22 0.55))
  (Game|SpawnActorfromClass "/Game/Mechanics/BP_SandChunk.BP_SandChunk_C" (Math|Transform|MakeTransform (Math|Vector|MakeVector (.x _returnvalue) (Math|Random|RandomFloatinRange (.y (Transformation|GetWorldLocation (Variables|Default|GetRightSpawnerLimit))) (.y (Transformation|GetWorldLocation (Variables|Default|GetLeftSpawnerLimit)))) (.z _returnvalue)) "0, 0, 0" (Math|Vector|MakeVector _returnvalue_2 _returnvalue_2 _returnvalue_2)) "Undefined" 0 0))

(event EventBeginPlay
  (Utilities|FlowControl|Delay 2.0)
  (Input|EnableInput (Game|GetPlayerController 0))
  (Utilities|Time|SetTimerbyEvent (delegate Custom|SpawnSand) (Variables|Default|GetSpawnRate) true))

(event Collision|EventActorBeginOverlap
  (params (OtherActor :type Actor%20Object%20Reference)))

(event EventTick
  (params (DeltaSeconds :type Float%20%28single-precision%29)))

(fn ConstructionScript
  (bind _distancefromcenter (Variables|Default|GetDistanceFromCenter))
  (bind _returnvalue (AddComponent|AddStaticMeshComponent false (Math|Transform|MakeTransform (Math|Vector|MakeVector 0.0 _distancefromcenter 0.0) "0, 0, 0" "1,1,1")))
  (bind _returnvalue_2 (AddComponent|AddStaticMeshComponent false (Math|Transform|MakeTransform (Math|Vector|MakeVector 0.0 (* _distancefromcenter -1.0) 0.0) "0, 0, 0" "1,1,1")))
  (Variables|Default|SetLeftSpawnerLimit _returnvalue)
  (Variables|Default|SetRightSpawnerLimit _returnvalue_2))

(fn ChangeDistancefromCenter
  (params (NewDistanceFromCenter :type Float%20%28single-precision%29))
  (Transformation|SetRelativeLocation (Variables|Default|GetLeftSpawnerLimit) (Math|Vector|MakeVector 0.0 NewDistanceFromCenter 0.0) false false)
  (Transformation|SetRelativeLocation (Variables|Default|GetRightSpawnerLimit) (Math|Vector|MakeVector 0.0 (* NewDistanceFromCenter -1.0) 0.0) false false))